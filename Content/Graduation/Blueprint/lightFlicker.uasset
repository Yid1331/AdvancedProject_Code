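; Light flicker actor that makes its SpotLight blink off at random intervals once activated.
; SetBoolean switches on the Overlapping flag, which nothing here clears or sets from an overlap event.
; While the flag is true, Tick shows the PointLight, waits a random whole number of seconds, then hides the SpotLight briefly before showing it again.
; The latent Delays on Tick pace the repeating flicker without a timer or loop.
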(event EventBeginPlay)

(event Collision|EventActorBeginOverlap
  (params (OtherActor :type Actor%20Object%20Reference)))

(event EventTick
  (params (DeltaSeconds :type Float%20%28single-precision%29))
  (bind _spotlight (Variables|Default|GetSpotLight))
  (if (Variables|Default|GetOverlapping?)
    (Rendering|SetVisibility (Variables|Default|GetPointLight) true false)
    (Utilities|FlowControl|Delay (Math|Conversions|ToFloat(Integer) (Math|Random|RandomInteger 6)))
    (Rendering|SetVisibility _spotlight false false)
    (Utilities|FlowControl|Delay 0.2)
    (Rendering|SetVisibility _spotlight true false)))

(fn ConstructionScript)

(fn SetBoolean
  (Variables|Default|SetOverlapping? true))