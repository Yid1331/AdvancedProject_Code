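; TreeLight is a Blueprint that shows or hides a particle system and a point light, depending on a BoxCollision flag.
; Every Tick polls the flag and sets the visibility of both components to match, without propagating to children.
; A BoxCollision? function sets the flag to true; nothing in this Blueprint calls it or resets the flag.
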(event EventTick
  (params (DeltaSeconds :type Float%20%28single-precision%29))
  (if (Variables|Default|GetBoxCollision)
    (Rendering|SetVisibility (Variables|Default|GetParticleSystem) true false)
    (Rendering|SetVisibility (Variables|Default|GetPointLight) true false)
    (else
      (Rendering|SetVisibility (Variables|Default|GetParticleSystem) false false)
      (Rendering|SetVisibility (Variables|Default|GetPointLight) false false))))

(fn ConstructionScript)

(fn BoxCollision?
  (Variables|Default|SetBoxCollision true))