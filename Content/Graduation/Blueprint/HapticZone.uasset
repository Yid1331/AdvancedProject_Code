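; HapticZone is a trigger volume that makes the player's motion controllers vibrate while something overlaps its box.
; Begin overlap starts a looping haptic effect on both hands through the first player controller, and end overlap stops both.
; The overlap events do not filter which actor entered, and the helper that derives a hand from the controller's motion source is unused.
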(event OnComponentBeginOverlap(Box)
  (params (OverlappedComponent :type Primitive%20Component%20Object%20Reference) (OtherActor :type Actor%20Object%20Reference) (OtherComp :type Primitive%20Component%20Object%20Reference) (OtherBodyIndex :type Integer) (bFromSweep :type Boolean) (SweepResult :type Hit%20Result%20Structure%20%28by%20ref%29))
  (Utilities|FlowControl|Sequence
    (:then_0
      (Variables|Default|SetMotion%20Controller%20Ref (Variables|Default|GetMotionController))
      (Class|PlayerController|PlayHapticEffect (Game|GetPlayerController 0) (Variables|Default|GetOnGrabHapticEffect) "Left" 1.0 true))
    (:then_1
      (Variables|Default|SetMotion%20Controller%20Ref (Variables|Default|GetMotionController))
      (Class|PlayerController|PlayHapticEffect (Game|GetPlayerController 0) (Variables|Default|GetOnGrabHapticEffect) "Right" 1.0 true))))

(event OnComponentEndOverlap(Box)
  (params (OverlappedComponent :type Primitive%20Component%20Object%20Reference) (OtherActor :type Actor%20Object%20Reference) (OtherComp :type Primitive%20Component%20Object%20Reference) (OtherBodyIndex :type Integer))
  (Utilities|FlowControl|Sequence
    (:then_0
      (Variables|Default|SetMotion%20Controller%20Ref (Variables|Default|GetMotionController))
      (Class|PlayerController|StopHapticEffect (Game|GetPlayerController 0) "Left"))
    (:then_1
      (Variables|Default|SetMotion%20Controller%20Ref (Variables|Default|GetMotionController))
      (Class|PlayerController|StopHapticEffect (Game|GetPlayerController 0) "Right"))))

(fn ConstructionScript)