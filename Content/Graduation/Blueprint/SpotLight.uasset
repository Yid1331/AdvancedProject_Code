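; SpotLight is a flickering light Blueprint with a spot light and a point light, switched on by an Overlapping flag.
; Set Boolean raises the flag, and nothing in this file clears it.
; While it is set, Tick shows the point light, waits a random few seconds, then briefly hides the spot light and plays a 2D flicker sound as it returns.
; Latent Delays inside Tick pace the repeating flicker.
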(event EventBeginPlay)

(event Collision|EventActorBeginOverlap
  (params (OtherActor :type Actor%20Object%20Reference)))

(event EventTick
  (params (DeltaSeconds :type Float%20%28single-precision%29))
  (bind _spotlight (Variables|Default|GetSpotLight))
  (if (Variables|Default|GetOverlapping?)
    (Rendering|SetVisibility (Variables|Default|GetPointLight) true false)
    (Utilities|FlowControl|Delay (Math|Conversions|ToFloat(Integer) (Math|Random|RandomInteger 6)))
    (Rendering|SetVisibility _spotlight false false)
    (Utilities|FlowControl|Delay 0.2)
    (Rendering|SetVisibility _spotlight true false)
    (Audio|PlaySound2D "/Game/Graduation/sound/FLICKER_SOUND_EFFECT_Cue.FLICKER_SOUND_EFFECT_Cue" 1.0 1.0 0.0 0 0)))

(fn ConstructionScript)

(fn SetBoolean
  (Variables|Default|SetOverlapping? true))